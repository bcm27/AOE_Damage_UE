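; AODamageGameState is a game state Blueprint with a SpawnAOE function that finds targets for area-of-effect hits around a location.
; It sphere-overlaps Pawns, excluding the instigator, and fires the caller's hit delegate for each actor implementing BPI_Health, with an optional debug sphere.
; The delegate is bound only for the duration of the call to prevent repeat hits.
; The RequireLOS input is currently unused.
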(fn `SpawnAOE`
  (params (Location :type "Vector Structure") (Radius :type "Float (double-precision)") (RequireLOS :type Boolean) (`AOE Instigator` :type "Actor Object Reference") (`Hit Delegate` :type "Delegate (by ref)") (DebugDrawDuration :type "Float (double-precision)") (DebugColor :type "LinearColor Structure"))
  (locals (OurCurrentActor :type "Actor Object Reference"))
  (add `self.AOE Hit Delegate` `Hit Delegate`)
  (`|ExecutionSequence`
    (:`then_0`
      (if (> (`local.DebugDrawDuration`) 0.0)
        (`KismetSystemLibrary.DrawDebugSphere` (`local.Location`) (`local.Radius`) 16 (`local.DebugColor`) (`local.DebugDrawDuration`) 2.0))
      (bind _outactors (`KismetSystemLibrary.SphereOverlapActors` (`local.Location`) (`local.Radius`) (`|MakeArray` "ObjectTypeQuery3" :!type "EObjectTypeQuery Enum") "/Script/Engine.Actor" (`|MakeArray` (`local.AOE Instigator`))))
      (for _array_element _outactors
        ;[1 1 1] Does the thing we hit implement health interface
        (bind _output_get (set `local.OurCurrentActor` _array_element))
        (if (`KismetSystemLibrary.DoesImplementInterface` _output_get "/Game/AOEDamage/Blueprints/Interfaces/BPI_Health.BPI_Health_C")
          (`self.AOE Hit Delegate` (`local.OurCurrentActor`)))))
    (:`then_1`
      ;[1 1 1] unbind all delegates so they dont repeat infinitly
      (remove `self.AOE Hit Delegate` `Hit Delegate`))))

(fn `UserConstructionScript`)